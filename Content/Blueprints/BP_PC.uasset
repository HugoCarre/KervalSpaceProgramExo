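; BP_PC, apparently a player controller, provides a helper that finds the world location under the mouse cursor.
; GetMouseLocation traces under the cursor against static and dynamic world objects, then projects along the deprojected mouse ray by the hit distance.
; That distance is capped at BP_Player's spring arm length, limiting the point's reach.
; The event graph and construction script contain no logic.
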(fn `Get mouse Location`
  (returns (Location :type "Vector Structure"))
  (bind _returnvalue (`GameplayStatics.GetPlayerController` 0))
  (bind (_worldlocation _worlddirection) (`self.DeprojectMousePositionToWorld` _returnvalue))
  (bind (_hitresult _returnvalue_2) (`self.GetHitResultUnderCursorForObjects` _returnvalue (`|MakeArray` "ObjectTypeQuery1" "ObjectTypeQuery2" :!type "EObjectTypeQuery Enum") true))
  (if _returnvalue_2
    (return (+ _worldlocation (* _worlddirection (`KismetMathLibrary.FClamp` (`.Distance` (`GameplayStatics.BreakHitResult` _hitresult)) 0.0 (`SpringArmComponent.TargetArmLength` (`/Game/Blueprints/BP_Player.SpringArm` (cast `/Game/Blueprints/BP_Player` (`GameplayStatics.GetPlayerPawn` 0) :!pure true)))))))))

(fn `UserConstructionScript`)