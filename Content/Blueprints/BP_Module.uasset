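; BP_Module is a mesh-based module actor that enables player input and highlights itself through custom depth while the cursor hovers over it.
; Initialization assigns the supplied static mesh, guarded by an IsInit flag that this file never sets.
; It then spawns a BP_Attach actor at every socket on the mesh and attaches it to the module, so socket layout defines the attach points.
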(event `self.ReceiveBeginPlay`
  (`self.EnableInput` (`GameplayStatics.GetPlayerController` 0)))

(event `self.ReceiveActorBeginCursorOver`
  (`PrimitiveComponent.SetRenderCustomDepth` (`self.StaticMesh`) true))

(event `self.ReceiveActorEndCursorOver`
  (`PrimitiveComponent.SetRenderCustomDepth` (`self.StaticMesh`) false))

(fn `CreateAttach`
  (for _array_element (`SceneComponent.GetAllSocketNames` (`self.StaticMesh`))
    (bind _returnvalue (`|SpawnActorFromClass` "/Game/Blueprints/BP_Attach.BP_Attach_C" (`KismetMathLibrary.Conv_VectorToTransform` (`SceneComponent.GetSocketLocation` (`self.StaticMesh`) _array_element)) "AlwaysSpawn" "OverrideRootScale" null null))
    (`self.K2_AttachToActor` _returnvalue self _array_element "KeepWorld" "KeepWorld" "KeepWorld" true)))

(fn `Initialization`
  (params (Mesh :type "StaticMesh Object Reference"))
  (if (not (`self.IsInit`))
    (`self.SetMesh` Mesh)
    (`self.CreateAttach`)))

(fn `SetMesh`
  (params (Mesh :type "StaticMesh Object Reference"))
  (`StaticMeshComponent.SetStaticMesh` (`self.StaticMesh`) Mesh))

(fn `UserConstructionScript`)