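; Player Blueprint for a rocket builder: drags modules with the mouse to assemble a rocket and controls a spring-arm camera.
; Tick handles orbit, vertical movement and zoom, and moves the dragged module to the cursor.
; On drop, the first module centers, while new ones snap via the closest module's nearest attach pair or are destroyed.
; Placed modules return to their start position, or are destroyed if dropped outside the destroy radius.
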(event `InputAction|LeftClick`
  (params (Key :type "Key Structure"))
  ;[1 1 1] Begin/End dragging
  (:`Pressed`
    (`/Engine/EditorBlueprintResources/StandardMacros.IsValid` (`self.DraggingModule`)
      (:`Is Valid`
        (`self.RemoveModuleToDrag`))
      (:`Is Not Valid`
        (for _array_element (`self.Modules`)
          (if (`/Game/Blueprints/BP_Module.IsCursorOver` _array_element)
            (`self.AddModuleToDrag` _array_element)))))))

(event `InputAction|LeftClick`
  (params (Key :type "Key Structure"))
  ;[1 1 1] Begin/End dragging
  (:`Pressed`
    (bind _isa (`/Engine/EditorBlueprintResources/StandardMacros.FlipFlop` :!label _label)
      (:`A`
        _)
      (:`B`
        _))
    (set `self.IsLeftClicking` _isa))
  (:`Released`
    (goto _label)))

(event `InputAction|RightClick`
  (params (Key :type "Key Structure"))
  ;[1 1 1] Turn around rocket
  (:`Pressed`
    (bind _isa (`/Engine/EditorBlueprintResources/StandardMacros.FlipFlop` :!label _label_2)
      (:`A`
        _)
      (:`B`
        _))
    (set `self.IsRightClicking` _isa))
  (:`Released`
    (goto _label_2)))

(event `InputAction|WheelClick`
  (params (Key :type "Key Structure"))
  ;[1 1 1] Move Up/Down
  (:`Pressed`
    (bind _isa (`/Engine/EditorBlueprintResources/StandardMacros.FlipFlop` :!label _label_3)
      (:`A`
        _)
      (:`B`
        _))
    (set `self.IsWheelClicking` _isa))
  (:`Released`
    (goto _label_3)))

(event `self.ReceiveTick`
  (params (DeltaSeconds :type "Float (single-precision)"))
  (bind _springarm (`self.SpringArm`))
  (`|ExecutionSequence`
    (:`then_0`
      ;[1 1 1] Turn around rocket
      (if (`self.IsRightClicking`)
        (`SceneComponent.K2_SetWorldRotation` (`self.SpringArm`) (`KismetMathLibrary.MakeRotator` (.roll (`SceneComponent.K2_GetComponentRotation` (`self.SpringArm`))) (`KismetMathLibrary.ClampAngle` (+ (.pitch (`SceneComponent.K2_GetComponentRotation` (`self.SpringArm`))) (* (`self.GetInputAxisValue`) 100.0 (`GameplayStatics.GetWorldDeltaSeconds`))) (- 360.0 75.0) 350.0) (+ (.yaw (`SceneComponent.K2_GetComponentRotation` (`self.SpringArm`))) (* (`self.GetInputAxisValue`) 100.0 (`GameplayStatics.GetWorldDeltaSeconds`)))) false false)))
    (:`then_1`
      ;[1 1 1] Move Up/Down
      (if (`self.IsWheelClicking`)
        (`SceneComponent.K2_SetWorldLocation` (`self.SpringArm`) (`KismetMathLibrary.MakeVector` (.x (`SceneComponent.K2_GetComponentLocation` (`self.SpringArm`))) (.y (`SceneComponent.K2_GetComponentLocation` (`self.SpringArm`))) (+ (.z (`SceneComponent.K2_GetComponentLocation` (`self.SpringArm`))) (* (`self.GetInputAxisValue`) 1000.0 (`GameplayStatics.GetWorldDeltaSeconds`)))) false false)))
    (:`then_2`
      ;[1 1 1] Zoom
      (set `SpringArmComponent.TargetArmLength` (`KismetMathLibrary.FClamp` (+ (* (`self.GetInputAxisValue`) 3000.0 (`GameplayStatics.GetWorldDeltaSeconds`)) (`SpringArmComponent.TargetArmLength` _springarm)) 500.0 2000.0) _springarm))
    (:`then_3`
      ;[1 1 1] Dragging Update and make object looking to rocket (correct rotation)
      (`/Engine/EditorBlueprintResources/StandardMacros.IsValid` (`self.DraggingModule`)
        (:`Is Valid`
          (`/Game/Blueprints/BP_Module.RotateToRocket` (`self.DraggingModule`))
          (`self.K2_SetActorLocation` (`self.DraggingModule`) (`KismetMathLibrary.MakeVector` (.x (`/Game/Blueprints/BP_PC.Get mouse Location` (cast `/Game/Blueprints/BP_PC` (`GameplayStatics.GetPlayerController` 0) :!pure true))) (.y (`/Game/Blueprints/BP_PC.Get mouse Location` (cast `/Game/Blueprints/BP_PC` (`GameplayStatics.GetPlayerController` 0) :!pure true))) (+ (.z (`/Game/Blueprints/BP_PC.Get mouse Location` (cast `/Game/Blueprints/BP_PC` (`GameplayStatics.GetPlayerController` 0) :!pure true))) (.z (`.Max` (break `Box` (`StaticMesh.GetBoundingBox` (`StaticMeshComponent.StaticMesh` (`/Game/Blueprints/BP_Module.StaticMesh` (`self.DraggingModule`))))))))) false false))))))

(fn `AddModuleToDrag`
  (params (ModuleToAttach :type "/Game/Blueprints/BP_Module Object Reference"))
  (bind _returnvalue (`GameplayStatics.GetPlayerController` 0))
  (bind (_locationx _locationy) (`PlayerController.GetMousePosition` _returnvalue))
  (bind (_worldposition _worlddirection) (`GameplayStatics.DeprojectScreenToWorld` _returnvalue (`KismetMathLibrary.MakeVector2D` _locationx _locationy)))
  (`/Engine/EditorBlueprintResources/StandardMacros.IsValid` (`self.DraggingModule`)
    (:`Is Valid`
      (`self.RemoveModuleToDrag`))
    (:`Is Not Valid`
      _))
  (bind _output_get (set `self.DraggingModule` ModuleToAttach))
  (`self.K2_SetActorLocation` _output_get (+ _worldposition (* _worlddirection (`SpringArmComponent.TargetArmLength` (`self.SpringArm`)))) false true)
  (`/Game/Blueprints/BP_Module.SetAttachesVisibility` _output_get true)
  (`PrimitiveComponent.SetCollisionObjectType` (`/Game/Blueprints/BP_Module.StaticMesh` _output_get) "ECC_Pawn"))

(fn `AddModuleToRocket`
  (params (Module :type "/Game/Blueprints/BP_Module Object Reference"))
  (`/Game/Blueprints/BP_Module.ActualizeStartPos` Module)
  (`KismetArrayLibrary.Array_Add` (`self.Modules`) Module)
  (`PrimitiveComponent.SetCollisionObjectType` (`/Game/Blueprints/BP_Module.StaticMesh` Module) "ECC_WorldDynamic"))

(fn `RemoveModuleToDrag`
  (bind _draggingmodule (`self.DraggingModule`))
  (bind _draggingmodule_2 (`self.DraggingModule`))
  (bind _draggingmodule_3 (`self.DraggingModule`))
  (`/Game/Blueprints/BP_Module.SetAttachesVisibility` (`self.DraggingModule`) false)
  (if (>= (`KismetArrayLibrary.Array_Length` (`self.Modules`)) 1)
    (if (`KismetArrayLibrary.Array_Contains` (`self.Modules`) (`self.DraggingModule`))
      (if (<= (`KismetMathLibrary.Vector_Distance2D` (`self.K2_GetActorLocation` (`self.DraggingModule`)) (`self.K2_GetActorLocation`)) (`self.DestroyRadius`))
        (`PrimitiveComponent.SetCollisionObjectType` (`/Game/Blueprints/BP_Module.StaticMesh` _draggingmodule_3) "ECC_WorldDynamic")
        (`self.K2_SetActorLocation` _draggingmodule_3 (`/Game/Blueprints/BP_Module.StartPos` _draggingmodule_3) false false)
        (set `self.DraggingModule` null)
        (else
          (`KismetArrayLibrary.Array_RemoveItem` (`self.Modules`) (`self.DraggingModule`))
          (`self.K2_DestroyActor` (`self.DraggingModule`))))
      (else
        (bind (_snapped _rocketattach _draggingattach) (`self.TrySnapModule`))
        (if _snapped
          (`/Game/Blueprints/BP_Module.SnapToRocket` _draggingmodule_2 (`self.K2_GetActorLocation` _rocketattach) (`self.K2_GetActorLocation` _draggingattach))
          (`self.AddModuleToRocket` _draggingmodule_2)
          (set `self.DraggingModule` null)
          (else
            (`self.K2_DestroyActor` (`self.DraggingModule`))))))
    (elif (<= (`KismetMathLibrary.Vector_Distance2D` (`self.K2_GetActorLocation` (`self.DraggingModule`)) (`self.K2_GetActorLocation`)) (`self.DestroyRadius`))
      (`self.K2_SetActorLocation` _draggingmodule (`KismetMathLibrary.MakeVector` 0.0 0.0 (.z (`self.K2_GetActorLocation` (`self.DraggingModule`)))) false true)
      (`self.AddModuleToRocket` _draggingmodule)
      (`PrimitiveComponent.SetCollisionObjectType` (`/Game/Blueprints/BP_Module.StaticMesh` (`self.DraggingModule`)) "ECC_WorldDynamic")
      (set `self.DraggingModule` null)
      (else
        (`self.K2_DestroyActor` (`self.DraggingModule`))))))

(fn `TrySnapModule`
  (returns (Snapped :type Boolean) (RocketAttach :type "/Game/Blueprints/BP_Attach Object Reference") (DraggingAttach :type "/Game/Blueprints/BP_Attach Object Reference"))
  (locals (ClosestRocketAttach :type "/Game/Blueprints/BP_Attach Object Reference") (ClosestDraggingAttach :type "/Game/Blueprints/BP_Attach Object Reference") (ClosestModule :type "/Game/Blueprints/BP_Module Object Reference") (DistanceMin :type "Float (double-precision)" :default 10000.0) (DistanceMinAttach :type "Float (double-precision)" :default 10000.0))
  (bind _closestmodule (`local.ClosestModule`))
  (`/Engine/EditorBlueprintResources/StandardMacros.IsValid` (`self.DraggingModule`)
    (:`Is Valid`
      ;[1 1 1] Get closest module to dragObject
      (for _array_element (`self.Modules`)
        (if (not (== _array_element (`self.DraggingModule`)))
          (bind _returnvalue (`KismetMathLibrary.Vector_Distance` (`self.K2_GetActorLocation` _array_element) (`self.K2_GetActorLocation` (`self.DraggingModule`))))
          (if (<= _returnvalue (`local.DistanceMin`))
            (set `local.ClosestModule` _array_element)
            (set `local.DistanceMin` _returnvalue))))
      (`/Engine/EditorBlueprintResources/StandardMacros.IsValid` _closestmodule
        (:`Is Valid`
          ;[1 1 1] Get Rocket Attach and dragging attach (closest)
          (for _array_element_2 (`/Game/Blueprints/BP_Module.Attaches` _closestmodule)
            (for _array_element_3 (`/Game/Blueprints/BP_Module.Attaches` (`self.DraggingModule`))
              (bind _returnvalue_2 (`KismetMathLibrary.Vector_Distance` (`self.K2_GetActorLocation` _array_element_3) (`self.K2_GetActorLocation` _array_element_2)))
              (if (and (<= _returnvalue_2 (`local.DistanceMinAttach`)) (<= _returnvalue_2 (`self.SnapRadius`)))
                (set `local.ClosestRocketAttach` _array_element_2)
                (set `local.ClosestDraggingAttach` _array_element_3)
                (set `local.DistanceMinAttach` _returnvalue_2))))
          (`/Engine/EditorBlueprintResources/StandardMacros.IsValid` (`local.ClosestRocketAttach`)
            (:`Is Valid`
              (`/Engine/EditorBlueprintResources/StandardMacros.IsValid` (`local.ClosestDraggingAttach`)
                (:`Is Valid`
                  (return true (`local.ClosestRocketAttach`) (`local.ClosestDraggingAttach`)))
                (:`Is Not Valid`
                  _)))
            (:`Is Not Valid`
              _)))
        (:`Is Not Valid`
          _)))
    (:`Is Not Valid`
      _))
  (return false null null))

(fn `UserConstructionScript`)